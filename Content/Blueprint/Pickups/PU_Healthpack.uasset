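; Health pack pickup Blueprint, built on a parent class, that hides itself when an actor tagged Player overlaps it.
; The overlap passes its sprite and itself to Hide, and the Restore event calls Show only if the pickup is respawnable.
; The construction script runs the parent's script, then clears the IsHealthTaken flag.
; No healing is applied in this graph.
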(event `self.ReceiveActorBeginOverlap`
  (params (OtherActor :type "Actor Object Reference"))
  (if (`self.ActorHasTag` OtherActor "Player")
    (`self.Hide` (`self.Sprite`) self)))

(event `self.Restore`
  (if (`self.Respawnable`)
    (`self.Show`)))

(fn `UserConstructionScript`
  (`parent.UserConstructionScript`)
  (set `self.is Health Taken` false))