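; Sword pickup Blueprint with a sprite that disappears when an actor tagged Player overlaps it.
; On overlap it hides the sprite, turns off its overlap events and adds itself to BP_Player's destroyed-actors record instead of being destroyed.
; Restore reverses the hide and re-enables overlaps only when Respawnable is set.
; The construction script runs the parent's, then stores the component's sprite in ActorSprite.
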(event `self.ReceiveActorBeginOverlap`
  (params (OtherActor :type "Actor Object Reference"))
  (if (`self.ActorHasTag` OtherActor "Player")
    (`SceneComponent.SetVisibility` (`self.Sprite`) false false)
    (set `PrimitiveComponent.bGenerateOverlapEvents` false (`self.Sprite`))
    (bind _asbp_player (cast `/Game/Blueprint/Player/BP_Player` (`GameplayStatics.GetPlayerCharacter` 0)))
    (`/Game/Blueprint/Player/BP_Player.Add To Destroyed Actors` _asbp_player self)))

(event `self.Restore`
  (if (`self.Respawnable`)
    (`SceneComponent.SetVisibility` (`self.Sprite`) true false)
    (set `PrimitiveComponent.bGenerateOverlapEvents` true (`self.Sprite`))))

(fn `UserConstructionScript`
  (`parent.UserConstructionScript`)
  (set `self.Actor Sprite` (`PaperSpriteComponent.GetSprite` (`self.Sprite`))))