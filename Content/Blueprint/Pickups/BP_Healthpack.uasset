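; BP_Healthpack is a sprite-based health pickup that the player takes by overlapping it.
; An overlap from a Player-tagged actor hides the sprite, sets IsHealthTaken to block repeat pickups, and registers the pack as a respawnable actor.
; Instead of being destroyed, the pack is reused through a Restore event that shows the sprite and clears the flag.
; No healing is applied in these graphs.
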(event `self.ReceiveActorBeginOverlap`
  (params (OtherActor :type "Actor Object Reference"))
  (if (and (`self.ActorHasTag` OtherActor "Player") (not (`self.is Health Taken`)))
    (`SceneComponent.SetVisibility` (`self.Sprite`) false false)
    (set `self.is Health Taken` true)
    (`self.Add to respawnable actors` self)))

(event `self.Restore`
  (`SceneComponent.SetVisibility` (`self.Sprite`) true false)
  (set `self.is Health Taken` false))

(fn `UserConstructionScript`
  (`parent.UserConstructionScript`)
  (set `self.is Health Taken` false))