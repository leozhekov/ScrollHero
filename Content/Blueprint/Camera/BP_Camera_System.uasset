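; Zone-based side-view camera actor that follows the player within a bounded area and becomes the active view when the player is inside it.
; Each tick moves the camera to the player's X and Z, clamped to BoundingBox, while keeping its depth on Y.
; The ActorCollision box triggers a blended view-target switch on player overlap, begin play or respawn, so multiple cameras can hand off.
; The construction script applies exposed transforms and extents to the camera and both boxes.
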(event `self.ReceiveTick`
  (params (DeltaSeconds :type "Float (single-precision)"))
  ;[1 1 1] Setting the camera location to follow the player
  (bind _returnvalue (`self.GetPlayerLocation`))
  (`SceneComponent.K2_SetWorldLocation` (`self.Camera`) _returnvalue false false))

(event `self.ReceiveBeginPlay`
  ;[1 1 1] Setting the camera to focus on the player
  ;;[0.6561 0.6855 1] Setting the camera on begin play or when the player has respawned. If there are more than one cameras, the camera that has the player in its collision box will be focused on the player.
  (bind _returnvalue (`self.is PlayerActorOverlapping` :!label _label))
  (if _returnvalue
    (`PlayerController.SetViewTargetWithBlend` (`GameplayStatics.GetPlayerController` 0) self (`self.BlendTime`) "VTBlend_Linear" 0.0 false :!label _label_2)))

(event `Player has respawned`
  ;[1 1 1] Setting the camera to focus on the player
  ;;[0.6561 0.6855 1] Setting the camera on begin play or when the player has respawned. If there are more than one cameras, the camera that has the player in its collision box will be focused on the player.
  (goto _label))

(event `self.ActorCollision.OnComponentBeginOverlap`
  (params (OverlappedComponent :type "PrimitiveComponent Object Reference") (OtherActor :type "Actor Object Reference") (OtherComp :type "PrimitiveComponent Object Reference") (OtherBodyIndex :type Integer) (bFromSweep :type Boolean) (SweepResult :type "HitResult Structure (by ref)"))
  ;[1 1 1] Setting the camera to focus on the player
  (if (`self.ActorHasTag` OtherActor "Player")
    (goto _label_2)))

(fn `GetPlayerLocation`
  (returns (ReturnValue :type "Vector Structure"))
  (bind (_returnvalue_x _returnvalue_y _returnvalue_z) (`KismetMathLibrary.BreakVector` (`self.K2_GetActorLocation` (`GameplayStatics.GetPlayerCharacter` 0))))
  (bind (_returnvalue_x_2 _returnvalue_y_2) (`KismetMathLibrary.BreakVector` (`SceneComponent.K2_GetComponentLocation` (`self.Camera`))))
  (bind (_origin _boxextent) (`KismetSystemLibrary.GetComponentBounds` (`self.BoundingBox`)))
  (bind (_returnvalue_x_3 _returnvalue_y_3 _returnvalue_z_2) (`KismetMathLibrary.BreakVector` (- _origin _boxextent)))
  (bind (_returnvalue_x_4 _returnvalue_y_4 _returnvalue_z_3) (`KismetMathLibrary.BreakVector` (+ _origin _boxextent)))
  (return (`KismetMathLibrary.MakeVector` (`KismetMathLibrary.FClamp` _returnvalue_x _returnvalue_x_3 _returnvalue_x_4) _returnvalue_y_2 (`KismetMathLibrary.FClamp` _returnvalue_z _returnvalue_z_2 _returnvalue_z_3))))

(fn `is PlayerActorOverlapping`
  (returns (ReturnValue :type Boolean))
  (return (== (`KismetArrayLibrary.Array_Length` (`PrimitiveComponent.GetOverlappingActors` (`self.ActorCollision`) "/Game/Blueprint/Player/BP_Player.BP_Player_C")) 1)))

(fn `UserConstructionScript`
  (bind _camera (`self.Camera`))
  (bind _boundingbox (`self.BoundingBox`))
  (bind _actorcollision (`self.ActorCollision`))
  (`|ExecutionSequence`
    (:`then_0`
      (`SceneComponent.K2_SetRelativeTransform` _camera (`self.CameraTransform`) false false)
      (`CameraComponent.SetFieldOfView` _camera 90.0))
    (:`then_1`
      (`SceneComponent.K2_SetRelativeTransform` _boundingbox (`self.BoundingBoxTransform`) false false)
      (`BoxComponent.SetBoxExtent` _boundingbox (`self.InnerBoxExtent`) true))
    (:`then_2`
      (`SceneComponent.K2_SetRelativeTransform` _actorcollision (`self.ActorCameraTransform`) false false)
      (`BoxComponent.SetBoxExtent` _actorcollision (`self.OuterBoxExtent`) true))))