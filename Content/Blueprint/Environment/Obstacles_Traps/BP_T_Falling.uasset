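; BP_T_Falling is an obstacle block that gives way shortly after an actor tagged Player overlaps it.
; The first overlap tints the sprite red, waits a response delay, then hides it, switches collision to overlap and registers the block for respawn.
; If respawnable, Restore re-arms it with its construction-time sprite, visibility and blocking collision, but leaves the tint unchanged.
; The crumbling animation is still a todo.
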(event `self.ReceiveActorBeginOverlap`
  (params (OtherActor :type "Actor Object Reference"))
  (if (and (`self.ActorHasTag` OtherActor "Player") (not (`self.Activated`)))
    ;[1 1 1] todo - crumbling animation
    (`PaperSpriteComponent.SetSpriteColor` (`self.Sprite`) (make `LinearColor` 1.0 0.0 0.0 1.0))
    (set `self.Activated` true)
    (`KismetSystemLibrary.Delay` (`self.Block Falling Response Time`))
    (`SceneComponent.SetVisibility` (`self.Sprite`) false false)
    (`PrimitiveComponent.SetCollisionProfileName` (`self.Sprite`) "OverlapAll")
    (`self.Add to respawnable actors` self)))

(event `self.Restore`
  (if (`self.Respawnable`)
    (set `self.Activated` false)
    (`PaperSpriteComponent.SetSprite` (`self.Sprite`) (`self.Default Sprite`))
    (`SceneComponent.SetVisibility` (`self.Sprite`) true false)
    (`PrimitiveComponent.SetCollisionProfileName` (`self.Sprite`) "BlockAllDynamic")))

(fn `UserConstructionScript`
  (`parent.UserConstructionScript`)
  (set `self.Default Sprite` (`PaperSpriteComponent.GetSprite` (`self.Sprite`))))