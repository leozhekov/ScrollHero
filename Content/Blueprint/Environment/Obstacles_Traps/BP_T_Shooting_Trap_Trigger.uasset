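; Trigger actor for a shooting trap, firing it when the player overlaps the trigger.
; On begin overlap with an actor tagged Player, it toggles its Sprite's visibility and calls FireTrap on the referenced Trap.
; On end overlap it toggles the Sprite again, so the sprite's visibility follows player entry and exit.
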(event `self.ReceiveActorBeginOverlap`
  (params (OtherActor :type "Actor Object Reference"))
  (if (`self.ActorHasTag` OtherActor "Player")
    (`SceneComponent.ToggleVisibility` (`self.Sprite`) false)
    (`/Game/Blueprint/Environment/Obstacles_Traps/BP_T_Shooting_Trap.Fire Trap` (`self.Trap`))))

(event `self.ReceiveActorEndOverlap`
  (params (OtherActor :type "Actor Object Reference"))
  (if (`self.ActorHasTag` OtherActor "Player")
    (`SceneComponent.ToggleVisibility` (`self.Sprite`) false)))

(fn `UserConstructionScript`)