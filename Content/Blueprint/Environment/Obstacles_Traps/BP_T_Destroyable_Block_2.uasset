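; Destroyable block obstacle that loses health when damaged and can be restored.
; Any damage lowers health at a tenth of its value; surviving blocks get a purple tint as a placeholder for crumbling sprites.
; At zero health it hides, switches to overlap collision and registers itself with the player's destroyed-actor list.
; Restore refills health and brings back the default sprite, cached at construction, with visibility and blocking collision.
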(event `self.ReceiveAnyDamage`
  (params (Damage :type "Float (single-precision)") (DamageType :type "DamageType Object Reference") (InstigatedBy :type "Controller Object Reference") (DamageCauser :type "Actor Object Reference"))
  (bind _output_get (set `self.Health` (`KismetMathLibrary.FClamp` (- (`self.Health`) (/ Damage 10.0)) 0.0 (`self.MaxHealth`))))
  (if (<= _output_get 0.0)
    (`SceneComponent.SetVisibility` (`self.Sprite`) false false)
    (`PrimitiveComponent.SetCollisionProfileName` (`self.Sprite`) "OverlapAll")
    (bind _asbp_player (cast `/Game/Blueprint/Player/BP_Player` (`GameplayStatics.GetPlayerCharacter` 0)))
    (`/Game/Blueprint/Player/BP_Player.Add To Destroyed Actors` _asbp_player self)
    (else
      (`PaperSpriteComponent.SetSpriteColor` (`self.Sprite`) (make `LinearColor` 0.5 0.0 0.5 1.0)))))

(event `self.Restore`
  (bind _sprite (`self.Sprite`))
  (set `self.Health` (`self.MaxHealth`))
  (`PaperSpriteComponent.SetSprite` (`self.Sprite`) (`self.Default Sprite`))
  (`SceneComponent.SetVisibility` _sprite true false)
  (`PrimitiveComponent.SetCollisionProfileName` _sprite "BlockAll"))

(fn `UserConstructionScript`
  (`parent.UserConstructionScript`)
  (set `self.Health` (`self.MaxHealth`))
  (set `self.Default Sprite` (`PaperSpriteComponent.GetSprite` (`self.Sprite`))))