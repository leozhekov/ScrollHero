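; BP_Dagger is a dagger weapon actor that damages tagged actors it overlaps and then destroys itself.
; On overlap it switches on the other actor's first tag only.
; Enemy and T Destroyable targets receive the Damage value before the dagger is destroyed, while Terrain destroys it without dealing damage.
; The construction script only calls the parent's.
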(event `self.ReceiveActorBeginOverlap`
  (params (OtherActor :type "Actor Object Reference"))
  (bind _output_get (set `self.Overlapped Actor` OtherActor))
  (bind _tags (`Actor.Tags` _output_get))
  (if (> (`KismetArrayLibrary.Array_Length` _tags) 0)
    (switch `name` (`|GetArrayItem` _tags)
      (:`Terrain`
        _)
      (:`Enemy`
        (`GameplayStatics.ApplyDamage` (`self.Overlapped Actor`) (`self.Damage`) null self :!label _label))
      (:`T_Destroyable`
        (goto _label)))
    (`self.K2_DestroyActor`)))

(fn `UserConstructionScript`
  (`parent.UserConstructionScript`))