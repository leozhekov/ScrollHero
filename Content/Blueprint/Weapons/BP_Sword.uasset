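; BP_Sword is a 2D sprite sword weapon that damages the enemy it overlaps when attacked with.
; Actor overlap events store the last entering actor tagged Enemy and clear it when any such actor leaves.
; Attack applies the Damage value to that stored actor if valid, with the sword as damage causer.
; The construction script runs the parent's, then assigns the sword sprite.
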(event `self.ReceiveActorBeginOverlap`
  (params (OtherActor :type "Actor Object Reference"))
  (if (`self.ActorHasTag` OtherActor "Enemy")
    (set `self.OverlappingActor` OtherActor)))

(event `self.ReceiveActorEndOverlap`
  (params (OtherActor :type "Actor Object Reference"))
  (if (`self.ActorHasTag` OtherActor "Enemy")
    (set `self.OverlappingActor` null)))

(fn `Attack`
  (bind _overlappingactor (`self.OverlappingActor`))
  (`/Engine/EditorBlueprintResources/StandardMacros.IsValid` _overlappingactor
    (:`Is Valid`
      (`GameplayStatics.ApplyDamage` _overlappingactor (`self.Damage`) null self))))

(fn `UserConstructionScript`
  (`parent.UserConstructionScript`)
  (`PaperSpriteComponent.SetSprite` (`self.Sprite`) "/Game/Sprites/Weapons/T_Sword_Sprite_0.T_Sword_Sprite_0"))