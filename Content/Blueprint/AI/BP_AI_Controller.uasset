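; AI controller Blueprint that makes its pawn patrol back and forth between two target points.
; After a short delay on begin play, Patrol moves to the next point through a gate, swaps next and previous points, waits a retriggerable delay, then repeats.
; StopPatrol halts movement and closes the gate to break the loop.
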(event `self.ReceiveBeginPlay`
  ;[1 1 1] Begin play
  (`KismetSystemLibrary.Delay` 0.2)
  (`self.Patrol`))

(event `Patrol`
  (`|ExecutionSequence`
    (:`then_0`
      (goto _label :!via `Open`))
    (:`then_1`
      (`/Engine/EditorBlueprintResources/StandardMacros.Gate` true :!label _label
        (:`Exit`
          (`AITask_MoveTo.AIMoveTo` self (0.0 0.0 0.0) (`self.Next Target Point`) -1.0 "Default" "Default" false false
            (:`then`
              (`self.Switch Target Points`)
              (`KismetSystemLibrary.RetriggerableDelay` (`self.Patrol Delay duration`))
              (`self.Patrol`))))))))

(event `Stop Patrol`
  (`self.StopMovement`)
  (goto _label :!via `Close`))

(fn `UserConstructionScript`)