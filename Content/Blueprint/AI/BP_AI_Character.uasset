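; AI enemy character that damages the player on contact and can be killed by Sword- or Dagger-tagged damage causers.
; BeginPlay hands two target points to BP_AI_Controller and initializes the health bar widget.
; Incoming damage is divided by 100 before reducing health; at zero, movement stops and the actor is destroyed after a delay.
; Tick flips facing by X velocity, keeping the last direction when stationary, and rotates the health bar to match.
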(event `self.ReceiveHit`
  (params (MyComp :type "PrimitiveComponent Object Reference") (Other :type "Actor Object Reference") (OtherComp :type "PrimitiveComponent Object Reference") (bSelfMoved :type Boolean) (HitLocation :type "Vector Structure") (HitNormal :type "Vector Structure") (NormalImpulse :type "Vector Structure") (Hit :type "HitResult Structure (by ref)"))
  ;[1 1 1] Being touched by the player character
  (if (`self.ActorHasTag` Other "Player")
    (`GameplayStatics.ApplyPointDamage` Other 10.0 HitLocation Hit null self)))

(event `self.ReceiveAnyDamage`
  (params (Damage :type "Float (single-precision)") (DamageType :type "DamageType Object Reference") (InstigatedBy :type "Controller Object Reference") (DamageCauser :type "Actor Object Reference"))
  ;[1 1 1] Receiving damage.
  (if (or (`self.ActorHasTag` DamageCauser "Sword") (`self.ActorHasTag` DamageCauser "Dagger"))
    (`self.Modify Health` Damage)
    (if (<= (`self.Health`) 0.0)
      (`CharacterMovementComponent.DisableMovement` (`self.CharacterMovement`))
      (`KismetSystemLibrary.Delay` 1.0)
      (`self.K2_DestroyActor`))))

(event `self.ReceiveBeginPlay`
  ;[1 1 1] BeginPLay
  (`|ExecutionSequence`
    (:`then_1`
      (bind _asbp_ai_controller (cast `/Game/Blueprint/AI/BP_AI_Controller` (`AIBlueprintHelperLibrary.GetAIController` self)))
      (set `/Game/Blueprint/AI/BP_AI_Controller.Target Point 1` (`self.TargetPoint 1`) _asbp_ai_controller)
      (set `/Game/Blueprint/AI/BP_AI_Controller.Target Point 2` (`self.TargetPoint 2`) _asbp_ai_controller)
      (`self.Setup Healthbar`))))

(event `self.ReceiveTick`
  (params (DeltaSeconds :type "Float (single-precision)"))
  ;[1 1 1] Tick - Updates animation
  (`/Engine/EditorBlueprintResources/StandardMacros.CompareFloat` (.x (`MovementComponent.Velocity` (`self.GetMovementComponent`)))
    (:`>`
      (set `self.bisMovingRight` true)
      (`Controller.SetControlRotation` (`self.GetController`) (`KismetMathLibrary.MakeRotator` 0.0) :!label _label)
      (`SceneComponent.K2_SetRelativeRotation` (`self.Health Bar Component`) (struct :`Yaw` 90.0) false false))
    (:`==`
      (if (`self.bisMovingRight`)
        (goto _label)
        (else
          (`Controller.SetControlRotation` (`self.GetController`) (`KismetMathLibrary.MakeRotator` 0.0 0.0 180.0) :!label _label_2)
          (`SceneComponent.K2_SetRelativeRotation` (`self.Health Bar Component`) (struct :`Yaw` -90.0) false false))))
    (:`<`
      (set `self.bisMovingRight` false)
      (goto _label_2))))

(fn `Modify Health`
  (params (Damage :type "Float (double-precision)"))
  (bind _output_get (set `self.Health` (`KismetMathLibrary.FClamp` (- (`self.Health`) (/ Damage 100.0)) 0.0 (`self.MaxHealth`))))
  (`/Game/Blueprint/AI/AI_Health_Bar.Update Health` (`self.Healthbar`) _output_get))

(fn `Setup Healthbar`
  (bind _asai_health_bar (cast `/Game/Blueprint/AI/AI_Health_Bar` (`WidgetComponent.GetUserWidgetObject` (`self.Health Bar Component`))))
  (bind _output_get (set `self.Healthbar` _asai_health_bar))
  (set `/Game/Blueprint/AI/AI_Health_Bar.Health` (`self.Health`) _output_get)
  (set `/Game/Blueprint/AI/AI_Health_Bar.MaxHealth` (`self.MaxHealth`) (`self.HealthBar`))
  (`/Game/Blueprint/AI/AI_Health_Bar.Update Health` (`self.HealthBar`) (`self.Health`)))

(fn `UserConstructionScript`)