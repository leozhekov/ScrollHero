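; BP_Level_Database tracks changed actors in a level so they can be reset.
; It keeps lists of enemies, destroyed items and dropped items, with functions to register each and to unregister dropped items.
; ResetActors respawns the enemies, restores the destroyed items, destroys the dropped items, then clears all three lists.
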(fn `Add to destroyed items`
  (params (Destroyed :type "/Game/Blueprint/Common/BP_Respawnable Object Reference"))
  (`KismetArrayLibrary.Array_Add` (`self.Destroyed Items`) Destroyed))

(fn `Add to dropped items`
  (params (`Dropped item` :type "/Game/Blueprint/Common/BP_Respawnable Object Reference"))
  (`KismetArrayLibrary.Array_Add` (`self.Dropped items`) `Dropped item`))

(fn `Add to enemies`
  (params (Enemy :type "/Game/Blueprint/AI/BP_AI_Character Object Reference"))
  (`KismetArrayLibrary.Array_Add` (`self.Enemies`) Enemy))

(fn `Clear DB`
  (`KismetArrayLibrary.Array_Clear` (`self.Destroyed Items`))
  (`KismetArrayLibrary.Array_Clear` (`self.Dropped items`))
  (`KismetArrayLibrary.Array_Clear` (`self.Enemies`)))

(fn `Destroy dropped items`
  (for _array_element (`self.Dropped items`)
    (`self.K2_DestroyActor` _array_element)))

(fn `Remove from dropped items`
  (params (Dropped :type "/Game/Blueprint/Common/BP_Respawnable Object Reference"))
  (`KismetArrayLibrary.Array_RemoveItem` (`self.Dropped items`) Dropped))

(fn `Reset Actors`
  (`self.Respawn enemies`)
  (`self.Restore destroyed actors`)
  (`self.Destroy dropped items`)
  (`self.Clear DB`))

(fn `Respawn enemies`
  (for _array_element (`self.Enemies`)
    (`/Game/Blueprint/AI/BP_AI_Character.Respawn` _array_element))
  (return))

(fn `Restore destroyed actors`
  (for _array_element (`self.Destroyed Items`)
    (`/Game/Blueprint/Common/BP_Respawnable.Restore` _array_element))
  (return))

(fn `UserConstructionScript`)