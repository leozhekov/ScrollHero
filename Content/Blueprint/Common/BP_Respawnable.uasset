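; BP_Respawnable is a common actor Blueprint for sprite-based objects that are hidden and shown again instead of destroyed.
; Hide turns off a sprite's visibility and overlaps, then registers the given actor in BP_Player's destroyed-actors list; Show re-enables both.
; Spawned hides non-respawnable instances after a delay and disables their collision, without registering them.
; Restore is an empty function.
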(event `Spawned`
  (if (not (`self.Respawnable`))
    (`KismetSystemLibrary.Delay` 5.0)
    (`PrimitiveComponent.SetCollisionProfileName` (`self.Sprite`) "NoCollision")
    (`SceneComponent.SetVisibility` (`self.Sprite`) false false)
    (set `PrimitiveComponent.bGenerateOverlapEvents` false (`self.Sprite`))))

(fn `Add to respawnable actors`
  (params (Actor :type "/Game/Blueprint/Common/BP_Respawnable Object Reference"))
  (bind _asbp_player (cast `/Game/Blueprint/Player/BP_Player` (`GameplayStatics.GetPlayerCharacter` 0)))
  (`/Game/Blueprint/Player/BP_Player.Add To Destroyed Actors` _asbp_player Actor))

(fn `Hide`
  (params (Sprite :type "PaperSpriteComponent Object Reference") (Actor :type "/Game/Blueprint/Common/BP_Respawnable Object Reference"))
  (`SceneComponent.SetVisibility` Sprite false false)
  (set `PrimitiveComponent.bGenerateOverlapEvents` false Sprite)
  (`self.Add to respawnable actors` Actor))

(fn `Restore`)

(fn `Show`
  (`SceneComponent.SetVisibility` (`self.Sprite`) true false)
  (set `PrimitiveComponent.bGenerateOverlapEvents` true (`self.Sprite`)))

(fn `UserConstructionScript`)